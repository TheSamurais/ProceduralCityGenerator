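; Procedural building actor that assembles a grid-based block from modular instanced meshes in the Construction Script, sized by Width, Length and NumberOfFloors.
; Nested loops stack Corner pieces at the four corners, Foundation across the ground level and edge-rotated Floor pieces around the perimeter of upper levels.
; Piece spacing comes from mesh local bounds, while a final pass tiles Roof instances above the top level on a fixed-size grid.
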(event `self.ReceiveBeginPlay`)

(fn `UserConstructionScript`
  (locals (WallXBound :type "Float (double-precision)" :default 0.0) (WallYBound :type "Float (double-precision)" :default 0.0) (WallZBound :type "Float (double-precision)" :default 0.0))
  (set `local.WallXBound` (.x (* (`.Max` (`StaticMeshComponent.GetLocalBounds` (`self.Floor`))) 2)))
  (set `local.WallYBound` (.y (* (`.Max` (`StaticMeshComponent.GetLocalBounds` (`self.Floor`))) 2)))
  (set `local.WallZBound` (.z (* (`.Max` (`StaticMeshComponent.GetLocalBounds` (`self.Floor`))) 2)))
  (for _index (range (+ (`self.Width`) 1))
    (for _index_2 (range (+ (`self.Length`) 1))
      (if (== _index_2 0)
        (set `self.RotatorZ` 90.0))
      (if (== _index_2 (`self.Length`))
        (set `self.RotatorZ` 270.0))
      (if (== _index 0)
        (set `self.RotatorZ` 180.0))
      (if (== _index (`self.Width`))
        (set `self.RotatorZ` 0.0))
      (for _index_3 (range (+ (`self.NumberOfFloors`) 1))
        (bind _returnvalue (== _index_2 0))
        (bind _returnvalue_2 (== _index 0))
        (bind _returnvalue_3 (== _index (`self.Width`)))
        (bind _returnvalue_4 (== _index_2 (`self.Length`)))
        (if (and (or (and _returnvalue _returnvalue_2) (and _returnvalue _returnvalue_3) (and _returnvalue_4 _returnvalue_2) (and _returnvalue_4 _returnvalue_3)) (> (`self.Width`) 0) (> (`self.Length`) 0))
          (`InstancedStaticMeshComponent.AddInstance` (`self.Corner`) (`KismetMathLibrary.MakeTransform` (`KismetMathLibrary.MakeVector` (* _index (.x (* (`.Max` (`StaticMeshComponent.GetLocalBounds` (`self.Corner`))) 2))) (* _index_2 (.y (* (`.Max` (`StaticMeshComponent.GetLocalBounds` (`self.Corner`))) 2))) (* _index_3 (.z (* (`.Max` (`StaticMeshComponent.GetLocalBounds` (`self.Corner`))) 2))))) false)
          (elif (== _index_3 0)
            (`InstancedStaticMeshComponent.AddInstance` (`self.Foundation`) (`KismetMathLibrary.MakeTransform` (`KismetMathLibrary.MakeVector` (* _index (.x (* (`.Max` (`StaticMeshComponent.GetLocalBounds` (`self.Foundation`))) 2))) (* _index_2 (.y (* (`.Max` (`StaticMeshComponent.GetLocalBounds` (`self.Foundation`))) 2))) (* _index_3 (.z (* (`.Max` (`StaticMeshComponent.GetLocalBounds` (`self.Foundation`))) 2))))) false)
            (elif (or (== _index 0) (== _index (`self.Width`)) (== _index_2 0) (== _index_2 (`self.Length`)))
              (`InstancedStaticMeshComponent.AddInstance` (`self.Floor`) (`KismetMathLibrary.MakeTransform` (`KismetMathLibrary.MakeVector` (* _index (.x (* (`.Max` (`StaticMeshComponent.GetLocalBounds` (`self.Corner`))) 2))) (* _index_2 (.y (* (`.Max` (`StaticMeshComponent.GetLocalBounds` (`self.Corner`))) 2))) (* _index_3 (.z (* (`.Max` (`StaticMeshComponent.GetLocalBounds` (`self.Corner`))) 2)))) (`KismetMathLibrary.MakeRotator` 0.0 0.0 (`self.RotatorZ`))) false)))))))
  (for _index_4 (range (+ (`self.Width`) 1))
    (for _index_5 (range (+ (`self.Length`) 1))
      (`InstancedStaticMeshComponent.AddInstance` (`self.Roof`) (`KismetMathLibrary.MakeTransform` (`KismetMathLibrary.MakeVector` (* _index_4 256.0) (* _index_5 256.0) (* (+ (`self.NumberOfFloors`) 1) 256.0))) false))))