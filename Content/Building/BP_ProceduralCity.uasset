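; Procedural city actor that spawns a grid of BP_ProceduralBuildingSample buildings at BeginPlay and destroys them when it is destroyed.
; Nested loops over SizeX and SizeY place buildings at fixed spacing with seeded random jitter, skipping colliding spawns.
; GetNextBuildingHeight sets each floor count, either randomly from a stream or tapering with distance from an offsettable city center.
; Disconnected step nodes hold simpler versions of the spawn logic.
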(event `self.ReceiveTick`
  (params (DeltaSeconds :type "Float (single-precision)")))

(event `self.ReceiveBeginPlay`
  ;[1 1 1] Step 3
  (set `self.MaxCitySize` (make `IntPoint` (`self.SizeX`) (`self.SizeY`)))
  (for _index (range (`self.SizeX`))
    (set `self.WidthIndex` _index)
    (for _index_2 (range (`self.SizeY`))
      (set `self.LengthIndex` _index_2)
      (bind _returnvalue (`self.GetNextBuildingHeight` (`self.LengthIndex`) (`self.WidthIndex`)))
      (set `self.TempHeight` _returnvalue)
      (bind _output_get (set `self.RandomPositionOffset` (`KismetMathLibrary.RandomIntegerInRangeFromStream` -100 100 (`self.OffsetStream`))))
      (set `self.RandomWallNumber` (`KismetMathLibrary.RandomIntegerFromStream` 2 (`self.NewBuildingStream`)))
      (bind _returnvalue_2 (`|SpawnActorFromClass` "/Game/Building/BP_ProceduralBuildingSample.BP_ProceduralBuildingSample_C" (`KismetMathLibrary.MakeTransform` (+ (`SceneComponent.K2_GetComponentLocation` (`self.DefaultSceneRoot`)) (`KismetMathLibrary.MakeVector` (`KismetMathLibrary.Conv_IntToDouble` (- (* (`self.WidthIndex`) 1450) _output_get)) (`KismetMathLibrary.Conv_IntToDouble` (- (* (`self.LengthIndex`) 1450) _output_get))))) "DontSpawnIfColliding" "OverrideRootScale" null (`self.TempHeight`) 1 1 (`self.NewBuildingStream`) null))
      (`KismetArrayLibrary.Array_Add` (`self.Buildings`) _returnvalue_2))))

(event `self.ReceiveDestroyed`
  ;[1 1 1] Step 3
  (for _array_element (`self.Buildings`)
    (`self.K2_DestroyActor` _array_element)))

(fn `GetNextBuildingHeight`
  (params (LengthIndex :type Integer) (WidthIndex :type Integer))
  (returns (ReturnValue :type Integer))
  (locals (MaxHeight :type Integer) (NewHeight :type Integer))
  (bind _height (`self.Height`))
  (bind (_x _y) (break `IntPoint` (`self.MaxCitySize`)))
  (bind (_x_2 _y_2) (break `IntPoint` (`self.OffsetCenter`)))
  (if (`self.RandomHeight`)
    (set `local.NewHeight` (`KismetMathLibrary.Clamp` _height 0 (`KismetMathLibrary.RandomIntegerFromStream` _height (`self.NewBuildingHeightStream`))))
    (else
      (set `local.NewHeight` (`KismetMathLibrary.Clamp` (- _height (`KismetMathLibrary.Round` (`KismetMathLibrary.VSize2D` (`KismetMathLibrary.MakeVector2D` (`KismetMathLibrary.Conv_IntToDouble` (- (/ _x 2) (+ (`local.WidthIndex`) _x_2))) (`KismetMathLibrary.Conv_IntToDouble` (- (/ _y 2) (+ (`local.LengthIndex`) _y_2))))))) 0 _height))))
  (return (`local.NewHeight`)))

(fn `UserConstructionScript`)