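; Sample actor that procedurally builds the rectangular shell of a multi-floor building on BeginPlay from floor count, width and length.
; Each floor loops over four sides, adding a rotated corner instance followed by wall instances.
; RandomWallMesh picks one of two wall instance components per segment from a random stream.
; GetWallSize and GetCornerSize derive offsets from mesh bounds; unconnected earlier drafts remain in the construction script.
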(event `self.ReceiveBeginPlay`
  (bind (_width _height) (`self.GetWallSize`))
  (bind (_width_2 _height_2) (`self.GetWallSize`))
  (bind (_width_3 _height_3) (`self.GetWallSize`))
  (bind (_x _y _z) (`self.GetCornerSize` false true))
  (bind (_x_2 _y_2 _z_2) (`self.GetCornerSize` false true))
  (bind (_x_3 _y_3 _z_3) (`self.GetCornerSize` true))
  (bind (_min _max) (`StaticMeshComponent.GetLocalBounds` (`self.WallMesh`)))
  (bind _returnvalue (+ (* (`self.Width`) _width_2) _y))
  (bind _returnvalue_2 (- (* _width_3 (`self.Length`) -1.0) _y_2))
  (for _index (range (+ (`self.NumberOfFloors`) 1))
    (set `self.RotatorZ` 0.0) ; Setting right angle for Yaw rotator
    (for _index_2 (range (+ (`self.Width`) 1))
      (if (== _index_2 0)
        (`InstancedStaticMeshComponent.AddInstance` (`self.Corner`) (`KismetMathLibrary.MakeTransform` (`KismetMathLibrary.MakeVector` 0.0 0.0 (* _index (`KismetMathLibrary.Abs` (.z (`.Max` (`StaticMeshComponent.GetLocalBounds` (`self.Corner`))))))) (`KismetMathLibrary.MakeRotator` 0.0 0.0 (`self.RotatorZ`))) false) ; Adding a corner instance
        (else
          (`self.RandomWallMesh`) ; Randoming mesh for wall (more info in macro)
          (`InstancedStaticMeshComponent.AddInstance` (`self.WallMesh`) (`KismetMathLibrary.MakeTransform` (`KismetMathLibrary.MakeVector` 0.0 (+ (.y (`.Max` (`StaticMeshComponent.GetLocalBounds` (`self.Corner`)))) (* (`KismetMathLibrary.Conv_IntToDouble` _index_2) (`KismetMathLibrary.Abs` (- (.y _min) (.y _max))))) (* _index (`KismetMathLibrary.Abs` (- (.z _min) (.z _max))))) (`KismetMathLibrary.MakeRotator` 0.0 0.0 (`self.RotatorZ`))) false) ; Adding previously randomed wall instance
        )))
    (set `self.RotatorZ` 90.0)
    (for _index_3 (range (+ (`self.Length`) 1))
      (if (== _index_3 0)
        (`InstancedStaticMeshComponent.AddInstance` (`self.Corner`) (`KismetMathLibrary.MakeTransform` (`KismetMathLibrary.MakeVector` 0.0 _returnvalue (* _index _z)) (`KismetMathLibrary.MakeRotator` 0.0 0.0 (`self.RotatorZ`))) false)
        (else
          (`self.RandomWallMesh`)
          (`InstancedStaticMeshComponent.AddInstance` (`self.WallMesh`) (`KismetMathLibrary.MakeTransform` (`KismetMathLibrary.MakeVector` (- _x (* (`KismetMathLibrary.Conv_IntToDouble` _index_3) _width_2)) _returnvalue (* _index _height_2)) (`KismetMathLibrary.MakeRotator` 0.0 0.0 (`self.RotatorZ`))) false))))
    (set `self.RotatorZ` 180.0)
    (for _index_4 (range (+ (`self.Width`) 1))
      (if (== _index_4 0)
        (`InstancedStaticMeshComponent.AddInstance` (`self.Corner`) (`KismetMathLibrary.MakeTransform` (`KismetMathLibrary.MakeVector` _returnvalue_2 (+ (* (`self.Width`) _width_3) _y_2) (* _index _z_2)) (`KismetMathLibrary.MakeRotator` 0.0 0.0 (`self.RotatorZ`))) false)
        (else
          (`self.RandomWallMesh`)
          (`InstancedStaticMeshComponent.AddInstance` (`self.WallMesh`) (`KismetMathLibrary.MakeTransform` (`KismetMathLibrary.MakeVector` _returnvalue_2 (+ (`.Y` (`self.GetCornerSize` false)) (* (`KismetMathLibrary.Conv_IntToDouble` (- _index_4 1)) _width_3)) (* _index _height_3)) (`KismetMathLibrary.MakeRotator` 0.0 0.0 (`self.RotatorZ`))) false))))
    (set `self.RotatorZ` 270.0)
    (for _index_5 (range (+ (`self.Length`) 1))
      (if (== _index_5 0)
        (`InstancedStaticMeshComponent.AddInstance` (`self.Corner`) (`KismetMathLibrary.MakeTransform` (`KismetMathLibrary.MakeVector` (- (* _width (`self.Length`) -1.0) _x_3) 0.0 (* _index _z_3)) (`KismetMathLibrary.MakeRotator` 0.0 0.0 (`self.RotatorZ`))) false)
        (else
          (`self.RandomWallMesh`)
          (`InstancedStaticMeshComponent.AddInstance` (`self.WallMesh`) (`KismetMathLibrary.MakeTransform` (`KismetMathLibrary.MakeVector` (- (`self.GetCornerSize` false) (* (`KismetMathLibrary.Conv_IntToDouble` (- _index_5 1)) _width)) 0.0 (* _index _height)) (`KismetMathLibrary.MakeRotator` 0.0 0.0 (`self.RotatorZ`))) false))))))

(fn `GetCornerSize`
  (params (`2X` :type Boolean) (`2Y` :type Boolean))
  (returns (X :type "Float (double-precision)") (Y :type "Float (double-precision)") (Z :type "Float (double-precision)"))
  (bind (_min _max) (`StaticMeshComponent.GetLocalBounds` (`self.Corner`)))
  (bind _x (.x _min))
  (bind _returnvalue (`KismetMathLibrary.Abs` (.y _max)))
  (return (`KismetMathLibrary.SelectFloat` (* (`KismetMathLibrary.Abs` _x) 2.0) _x (`local.2X`)) (`KismetMathLibrary.SelectFloat` (* _returnvalue 2.0) _returnvalue (`local.2Y`)) (.z _max)))

(fn `GetWallSize`
  (returns (Width :type "Float (double-precision)") (Height :type "Float (double-precision)"))
  (bind (_min _max) (`StaticMeshComponent.GetLocalBounds` (`self.WallMesh`)))
  (return (`KismetMathLibrary.Abs` (- (.y _min) (.y _max))) (`KismetMathLibrary.Abs` (- (.z _min) (.z _max)))))

(fn `UserConstructionScript`
  (locals (WallXBound :type "Float (double-precision)" :default 0.0) (WallYBound :type "Float (double-precision)" :default 0.0) (WallZBound :type "Float (double-precision)" :default 0.0)))